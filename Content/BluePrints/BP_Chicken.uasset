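; BP_Chicken is the player character of a Flappy Bird-style game, with flapping, scoring and death handling.
; BeginPlay loads or creates the HighscoreSave slot and shows the HUD.
; Jump or right mouse zeroes the physics capsule's velocity and applies an upward impulse while CanMove is true.
; Increasescore increments Score; any Hit disables flapping, swaps the flipbook, saves a new high score and shows the game-over widget with both scores.
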(event Custom|Increase%20score
  (Math|Integer|IncrementInt (Variables|Default|GetScore)))

(event EventBeginPlay
  (bind _returnvalue (Game|GetPlayerController 0))
  (Variables|/Script/Engine.PlayerController|SetbShowMouseCursor _returnvalue false)
  (Input|SetInputModeGameOnly _returnvalue false)
  (bind _returnvalue_2 (SaveGame|DoesSaveGameExist "1"))
  (if _returnvalue_2
    (bind _returnvalue_3 (SaveGame|LoadGamefromSlot "1"))
    (bind _ashighscore_save (Utilities|Casting|CastToHighscoreSave _returnvalue_3))
    (Variables|Default|SetAs%20Highscore%20Save _ashighscore_save)
    (else
      (bind _returnvalue_4 (SaveGame|CreateSaveGameObject "/Game/BluePrints/HighscoreSave.HighscoreSave_C"))
      (bind _output_get (Variables|Default|SetAs%20Highscore%20Save _returnvalue_4))
      (SaveGame|SaveGametoSlot _output_get "1")))
  (bind _returnvalue_5 (UserInterface|CreateWidget "/Game/BluePrints/BP_PlayerHUD.BP_PlayerHUD_C" 0 self))
  (bind _output_get_2 (Variables|Default|SetNewVar _returnvalue_5))
  (UserInterface|Viewport|AddtoViewport _output_get_2 0))

(event Collision|EventActorBeginOverlap
  (params (OtherActor :type Actor%20Object%20Reference)))

(event EventTick
  (params (DeltaSeconds :type Float%20%28single-precision%29)))

(event Collision|EventHit
  (params (MyComp :type Primitive%20Component%20Object%20Reference) (Other :type Actor%20Object%20Reference) (OtherComp :type Primitive%20Component%20Object%20Reference) (bSelfMoved :type Boolean) (HitLocation :type Vector :default "0, 0, 0") (HitNormal :type Vector :default "0, 0, 0") (NormalImpulse :type Vector :default "0, 0, 0") (Hit :type Hit%20Result%20Structure%20%28by%20ref%29))
  (bind _as_highscore_save (Variables|Default|GetAs%20Highscore%20Save))
  (Variables|Default|SetCan%20move false)
  (Sprite|SetFlipbook (Variables|Default|GetPaperFlipbook) "/Game/Assets/FlappyChickenAssets/T_TappyChicken_03.T_TappyChicken_03")
  (if (> (Variables|Default|GetScore) (Variables|/Game/BluePrints/HighscoreSave.HighscoreSave_C|Getsavedscore (Variables|Default|GetAs%20Highscore%20Save)))
    (Variables|/Game/BluePrints/HighscoreSave.HighscoreSave_C|Setsavedscore _as_highscore_save (Variables|Default|GetScore))
    (SaveGame|SaveGametoSlot _as_highscore_save "1"))
  (bind _returnvalue (UserInterface|CreateWidget "/Game/BluePrints/BP_GameOverScore.BP_GameOverScore_C"))
  (bind _output_get (Variables|Default|SetGameOverHud _returnvalue))
  (Rendering|Components|TextRender|SetText (Variables|/Game/BluePrints/BP_GameOverScore.BP_GameOverScore_C|Getplayerscore_1 _output_get) (Utilities|Text|ToText(Integer) (Variables|Default|GetScore)))
  (Rendering|Components|TextRender|SetText (Variables|/Game/BluePrints/BP_GameOverScore.BP_GameOverScore_C|Getplayerhighscore_1 _output_get) (Utilities|Text|ToText(Integer) (Variables|/Game/BluePrints/HighscoreSave.HighscoreSave_C|Getsavedscore (Variables|Default|GetAs%20Highscore%20Save))))
  (UserInterface|Viewport|AddtoViewport _output_get 0))

(event Input|ActionEvents|InputActionJump
  (params (Key :type Key%20Structure :default "None"))
  (bind _capsule (Variables|Default|GetCapsule))
  (:Pressed
    (if (Variables|Default|GetCan%20move)
      (Physics|SetPhysicsLinearVelocity _capsule "0, 0, 0" false "None")
      (Physics|AddImpulse _capsule "0.000000,0.000000,150.000000" "None" false))))

(event Input|MouseEvents|RightMouseButton
  (params (Key :type Key%20Structure :default "None"))
  (bind _capsule (Variables|Default|GetCapsule))
  (:Pressed
    (if (Variables|Default|GetCan%20move)
      (Physics|SetPhysicsLinearVelocity _capsule "0, 0, 0" false "None")
      (Physics|AddImpulse _capsule "0.000000,0.000000,150.000000" "None" false))))

(fn ConstructionScript)